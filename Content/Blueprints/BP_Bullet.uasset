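; BP_Bullet is a projectile actor that destroys enemies on contact.
; Each Tick it moves along its forward vector at MoveSpeed, scaled by delta time, using a non-swept location update.
; On overlap with a BP_Enermy, it destroys that enemy, spawns a P_Explosion particle effect at its own location and destroys itself, ignoring other actors.
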(event EventBeginPlay)

(event Collision|EventActorBeginOverlap
  (params (OtherActor :type Actor%20Object%20Reference))
  (bind _asbp_enermy (Utilities|Casting|CastToBP_Enermy OtherActor))
  (Actor|DestroyActor _asbp_enermy)
  (Effects|SpawnEmitteratLocation "/Game/StarterContent/Particles/P_Explosion.P_Explosion" (Transformation|GetActorLocation))
  (Actor|DestroyActor))

(event EventTick
  (params (DeltaSeconds :type Float%20%28single-precision%29))
  (Transformation|SetActorLocation (+ (Transformation|GetActorLocation) (* (* (Transformation|GetActorForwardVector) (Variables|속도|GetMoveSpeed)) DeltaSeconds)) false false))

(fn ConstructionScript)