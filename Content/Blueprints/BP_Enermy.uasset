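; BP_Enermy is an enemy actor that flies in a straight line and destroys the player on contact.
; On BeginPlay it picks a fixed direction: a 35% chance to aim at BP_Player's current position, otherwise its own forward vector, intended as downward.
; Tick moves it along that direction at MoveSpeed without sweeping.
; Overlapping BP_Player destroys the player, spawns an emitter at the enemy's location and destroys the enemy.
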(event EventBeginPlay
  (if (<= (Math|Random|RandomFloatinRange 0.0 1.0) 0.35)
    ;[1 1 1] 플레이어 향해
    (bind _returnvalue (Actor|GetActorOfClass "/Game/Blueprints/BP_Player.BP_Player_C"))
    (Utilities|IsValid _returnvalue
      (:Is%20Valid
        (Variables|Default|SetDirection (Math|Vector|Normalize (- (Transformation|GetActorLocation _returnvalue) (Transformation|GetActorLocation))))))
    (else
      ;[1 1 1] 밑으로 향해
      (Variables|Default|SetDirection (Transformation|GetActorForwardVector)))))

(event Collision|EventActorBeginOverlap
  (params (OtherActor :type Actor%20Object%20Reference))
  (bind _asbp_player (Utilities|Casting|CastToBP_Player OtherActor))
  (Actor|DestroyActor _asbp_player)
  (Effects|SpawnEmitteratLocation 0 (Transformation|GetActorLocation))
  (Actor|DestroyActor))

(event EventTick
  (params (DeltaSeconds :type Float%20%28single-precision%29))
  (Transformation|SetActorLocation (+ (Transformation|GetActorLocation) (* DeltaSeconds (* (Variables|Default|GetDirection) (Variables|Default|GetMoveSpeed)))) false false))

(fn ConstructionScript)